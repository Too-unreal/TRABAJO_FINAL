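; Base dialog component that runs branching conversations through a W_dialog widget added to the viewport.
; Dialog is an empty function, apparently for child overrides, in which each AddDialog call takes a speaker, text and options.
; Each selection is stored by step index and replays Dialog from the start: answered steps return their saved option, unanswered ones update the widget.
; Helpers close the widget, roll back steps or switch dialog tree, clearing progress.
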(event EventBeginPlay)

(event EventTick
  (params (DeltaSeconds :type Float%20%28single-precision%29)))

(fn StartDialog
  (bind _returnvalue (UserInterface|CreateWidget "/Game/UI/W_dialog.W_dialog_C" 0 self))
  (bind _output_get (Variables|Default|SetDialogWidget _returnvalue))
  (UserInterface|Viewport|AddtoViewport _output_get 0)
  (CallFunction|ProgressDialog))

(fn CloseDialog
  (Widget|RemovefromParent (Variables|Default|GetDialogWidget)))

(fn ProgressDialog
  (Variables|Default|SetDialogIndex -1)
  (CallFunction|Dialog))

(fn Dialog)

(fn AddDialog
  (params (Speaker :type Text) (Dialog :type Text) (Options :type Array%20of%20Texts))
  (bind _dialogprogress (Variables|Default|GetDialogProgress))
  (bind _dialogindex (Variables|Default|GetDialogIndex))
  (bind (_value _returnvalue) (Utilities|Map|Find _dialogprogress _dialogindex))
  (Math|Integer|IncrementInt (Variables|Default|GetDialogIndex)
    (:%20%20
      (if _returnvalue
        (return "NewEnumerator0" _value)
        (else
          (Default|UpdateDialogText (Variables|Default|GetDialogWidget) (Variables|Default|GetDialogIndex) Speaker Dialog Options)
          (return "NewEnumerator1" 0))))))

(fn UpdateSelectedOption
  (params (ProgressIndex :type Integer%20%28by%20ref%29) (OptionIndex :type Integer%20%28by%20ref%29))
  (Utilities|Map|Add (Variables|Default|GetDialogProgress) ProgressIndex OptionIndex)
  (CallFunction|ProgressDialog))

(fn ClearDialogProgress
  (Utilities|Map|Clear (Variables|Default|GetDialogProgress)))

(fn RemoveDialogProgress
  (params (ProgressSteps :type Integer))
  (for _index (range 0 ProgressSteps)
    (Utilities|Map|Remove (Variables|Default|GetDialogProgress) (- (Variables|Default|GetDialogIndex) _index))))

(fn SetDialogTreeIndex
  (params (DialogTreeIndex :type Integer))
  (Variables|Default|SetDialogTreeIndex DialogTreeIndex)
  (CallFunction|ClearDialogProgress))