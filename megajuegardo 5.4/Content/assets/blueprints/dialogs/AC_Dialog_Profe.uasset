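; Dialog component for the professor NPC "El MasCapo", holding his crude joke conversation in Spanish.
; It overrides Dialog and switches on DialogTreeIndex, chaining AddDialog nodes whose chosen options drive the branches.
; Early exits advance the tree to index 1, where he gives one of two random send-off lines.
; Following the joke to its end clears progress, closes the dialog and restarts the game through the Camara game mode.
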(event EventBeginPlay
  (|CallParentFunction) ; This node is disabled and will not be called.\nDrag off pins to build functionality.
)

(event EventTick
  (params (DeltaSeconds :type Float%20%28single-precision%29))
  (|CallParentFunction DeltaSeconds) ; This node is disabled and will not be called.\nDrag off pins to build functionality.
)

(fn Dialog
  (|CallParentFunction)
  (switch int (Variables|Default|GetDialogTreeIndex)
    (:0
      (bind (_state _optionindex) (CallFunction|AddDialog "El MasCapo" "El Masca Poronga. Pero me dicen Papito mi Rey " (Utilities|Array|MakeArray "Pero no pregunte nada" "OLEME EL DEDO")))
      (switch Utilities|FlowControl|Switch|SwitchonEnum_dialog _state
        (:NewEnumerator0
          (switch int _optionindex
            (:0
              (bind (_state_2 _optionindex_2) (CallFunction|AddDialog "El MasCapo" "ah, cierto, perdon, la costumbre " (Utilities|Array|MakeArray "Ta bien" "Nah mentira OLEME EL DEDO")))
              (switch Utilities|FlowControl|Switch|SwitchonEnum_dialog _state_2
                (:NewEnumerator0
                  (switch int _optionindex_2
                    (:0
                      (CallFunction|SetDialogTreeIndex 1)
                      (CallFunction|CloseDialog))
                    (:1
                      (bind (_state_3 _optionindex_3) (CallFunction|AddDialog "El MasCapo" "Mmmmmm... Tiene olor a... CHELE!" (Utilities|Array|MakeArray "Jaja un capo" "TIENE OLOR A GARCHA!") :!label _label))
                      (switch Utilities|FlowControl|Switch|SwitchonEnum_dialog _state_3
                        (:NewEnumerator0
                          (switch int _optionindex_3
                            (:0
                              (CallFunction|SetDialogTreeIndex 1)
                              (CallFunction|CloseDialog))
                            (:1
                              (bind (_state_4 _optionindex_4) (CallFunction|AddDialog "El MasCapo" "Ay, Se me hace agua la boca!" (Utilities|Array|MakeArray "Bueno Ya" "Y TIENE OLOR A ORTOOOO!")))
                              (switch Utilities|FlowControl|Switch|SwitchonEnum_dialog _state_4
                                (:NewEnumerator0
                                  (switch int _optionindex_4
                                    (:1
                                      (bind (_state_5 _optionindex_5) (CallFunction|AddDialog "El MasCapo" "MMMMMM!" (Utilities|Array|MakeArray "Bueno Ya" "Y TAMBIEN A ESCROTOOOOOO")))
                                      (switch Utilities|FlowControl|Switch|SwitchonEnum_dialog _state_5
                                        (:NewEnumerator0
                                          (switch int _optionindex_5
                                            (:1
                                              (bind _state_6 (CallFunction|AddDialog "El MasCapo" "MMM, me encanta" (Utilities|Array|MakeArray "Uhhh, la re puta madre")))
                                              (switch Utilities|FlowControl|Switch|SwitchonEnum_dialog _state_6
                                                (:NewEnumerator0
                                                  (CallFunction|ClearDialogProgress)
                                                  (CallFunction|CloseDialog)
                                                  (Utilities|FlowControl|DoOnce false
                                                    (:Completed
                                                      (bind _ascamara (Utilities|Casting|CastToCamara (Game|GetGameMode)))
                                                      (Default|RestartGame _ascamara))))))))))))))))))))))
            (:1
              (goto _label))))))
    (:1
      (bind _state_7 (CallFunction|AddDialog "El MasCapo" (Utilities|Select :Index (Math|Random|RandomIntegerinRange 0 1) :Option%200 "Bueno flaca, anda y matar monstuos" :Option%201 "Daaale, o queres que te bochen?") (Utilities|Array|MakeArray "ok")))
      (switch Utilities|FlowControl|Switch|SwitchonEnum_dialog _state_7
        (:NewEnumerator0
          (CallFunction|ClearDialogProgress)
          (CallFunction|CloseDialog))))))