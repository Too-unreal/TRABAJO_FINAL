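; Player character Blueprint for a 2D side-scrolling platformer, using a flipbook sprite of Chie.
; BeginPlay adds the Enhanced Input mapping context, which drives jumping and movement along world X.
; Movement input also snaps controller yaw to face left or right.
; Each Tick, Movete picks the idle, running, jump or fall flipbook from ground state and velocity.
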(event Input|EnhancedActionEvents|EnhancedInputActionsalto
  (params (ActionValue :type Boolean) (ElapsedSeconds :type Float%20%28double-precision%29) (TriggeredSeconds :type Float%20%28double-precision%29) (InputAction :type Input%20Action%20Object%20Reference :default "/Game/input/acciones/salto.salto"))
  (:Started
    (Character|Jump))
  (:Completed
    (Character|StopJumping)))

(event Input|EnhancedActionEvents|EnhancedInputActionmoverse
  (params (ActionValue :type Float%20%28double-precision%29) (ElapsedSeconds :type Float%20%28double-precision%29) (TriggeredSeconds :type Float%20%28double-precision%29) (InputAction :type Input%20Action%20Object%20Reference :default "/Game/input/acciones/moverse.moverse"))
  (Pawn|Input|AddMovementInput "1.000000,0.000000,0.000000" ActionValue false)
  (Pawn|SetControlRotation (Pawn|GetController) (select (> ActionValue 0.0) (Math|Rotator|MakeRotator 0.0 0.0 0.0) (Math|Rotator|MakeRotator 0.0 0.0 1.8e+02))))

(event EventBeginPlay
  (bind _asplayer_controller (Utilities|Casting|CastToPlayerController (Pawn|GetController)))
  (Input|AddMappingContext (PlayerController|LocalPlayerSubsystems|GetEnhancedInputLocalPlayerSubsystem _asplayer_controller) "/Game/input/plataformeo_mov.plataformeo_mov" 0 "(bIgnoreAllPressedKeysUntilRelease=True,bForceImmediately=False,bNotifyUserSettings=False)"))

(event Collision|EventActorBeginOverlap
  (params (OtherActor :type Actor%20Object%20Reference)))

(event EventTick
  (params (DeltaSeconds :type Float%20%28single-precision%29))
  (CallFunction|Movete))

(fn ConstructionScript)

(fn Movete
  (if (AI|Components|NavMovement|IsMovingonGround (Variables|Character|GetCharacterMovement))
    (if (> (Math|Vector|VectorLength (Transformation|GetVelocity)) 0.0)
      (Sprite|SetFlipbook (Variables|Default|GetSprite) "/Game/assets/Character/animations/chie_running.chie_running")
      (else
        (Sprite|SetFlipbook (Variables|Default|GetSprite) "/Game/assets/Character/animations/chie_idle.chie_idle")))
    (elif (< (.z (Transformation|GetVelocity)) -1e+02)
      (Sprite|SetFlipbook (Variables|Default|GetSprite) "/Game/assets/Character/animations/chie_fall.chie_fall")
      (else
        (Sprite|SetFlipbook (Variables|Default|GetSprite) "/Game/assets/Character/animations/chie_jump.chie_jump")))))