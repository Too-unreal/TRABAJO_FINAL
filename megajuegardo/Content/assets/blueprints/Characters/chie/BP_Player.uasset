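; BP_Player is the player character for a side-scrolling platformer, handling movement, jumping, attacking and pausing.
; It registers an Enhanced Input mapping context on BeginPlay, then moves along world X and flips control yaw to face the input direction.
; Attack plays an animation override in a slot, using an IsAttacking flag to block repeats until it completes or cancels.
; Pause opens the Pausa widget, switches to UI-only input and pauses the game.
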(event Input|EnhancedActionEvents|EnhancedInputActionsalto
  (params (ActionValue :type Boolean) (ElapsedSeconds :type Float%20%28double-precision%29) (TriggeredSeconds :type Float%20%28double-precision%29) (InputAction :type Input%20Action%20Object%20Reference :default "/Game/input/acciones/salto.salto"))
  (:Started
    (Character|Jump))
  (:Completed
    (Character|StopJumping)))

(event Input|EnhancedActionEvents|EnhancedInputActionmoverse
  (params (ActionValue :type Float%20%28double-precision%29) (ElapsedSeconds :type Float%20%28double-precision%29) (TriggeredSeconds :type Float%20%28double-precision%29) (InputAction :type Input%20Action%20Object%20Reference :default "/Game/input/acciones/moverse.moverse"))
  (Pawn|Input|AddMovementInput "1.000000,0.000000,0.000000" (.X (Math|Vector2D|BreakVector2D (Math|Conversions|ToVector2D(Vector) ActionValue))) false)
  (Pawn|SetControlRotation (Pawn|GetController) (select (> ActionValue 0.0) (Math|Rotator|MakeRotator 0.0 0.0 0.0) (Math|Rotator|MakeRotator 0.0 0.0 1.8e+02))))

(event Input|EnhancedActionEvents|EnhancedInputActionPAUSA
  (params (ActionValue :type Boolean) (ElapsedSeconds :type Float%20%28double-precision%29) (TriggeredSeconds :type Float%20%28double-precision%29) (InputAction :type Input%20Action%20Object%20Reference :default "/Game/input/acciones/PAUSA.PAUSA"))
  (bind _returnvalue (Game|GetPlayerController 0))
  (:Started
    (bind _returnvalue_2 (UserInterface|CreateWidget "/Game/UI/pausa.pausa_C"))
    (UserInterface|Viewport|AddtoViewport _returnvalue_2 0)
    (Variables|/Script/Engine.PlayerController|SetbShowMouseCursor _returnvalue true)
    (Input|SetInputModeUIOnly _returnvalue 0 "DoNotLock" false)
    (Game|SetGamePaused true)))

(event Input|EnhancedActionEvents|EnhancedInputActionAtaque
  (params (ActionValue :type Boolean) (ElapsedSeconds :type Float%20%28double-precision%29) (TriggeredSeconds :type Float%20%28double-precision%29) (InputAction :type Input%20Action%20Object%20Reference :default "/Game/input/acciones/Ataque.Ataque"))
  (:Started
    (if (not (Variables|Default|GetIsAttacking))
      (|PlayAnimationOverridewithCallbacks (Class|PaperZDCharacter|GetAnimInstance) "/Game/assets/blueprints/AnimSequences/attack1.attack1" "ataque" 1.0 0.0
        (:then
          (Variables|Default|SetIsAttacking true))
        (:OnCompleted
          (Variables|Default|SetIsAttacking false :!label _label))
        (:OnCancelled
          (goto _label))))))

(event EventBeginPlay
  (|CallParentFunction)
  (bind _asplayer_controller (Utilities|Casting|CastToPlayerController (Pawn|GetController)))
  (Input|AddMappingContext (PlayerController|LocalPlayerSubsystems|GetEnhancedInputLocalPlayerSubsystem _asplayer_controller) "/Game/input/plataformeo_mov.plataformeo_mov" 0 "(bIgnoreAllPressedKeysUntilRelease=True,bForceImmediately=False,bNotifyUserSettings=False)"))

(event Collision|EventActorBeginOverlap
  (params (OtherActor :type Actor%20Object%20Reference)))

(event EventTick
  (params (DeltaSeconds :type Float%20%28single-precision%29)))

(fn ConstructionScript
  (|CallParentFunction))