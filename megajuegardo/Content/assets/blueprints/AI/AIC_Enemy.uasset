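; AIC_Enemy is the AI controller for enemies, driving them with a behavior tree and blackboard.
; On BeginPlay it sets up BB_Enemy, runs BT_Enemy, and casts the first player pawn to BP_Player.
; That player is passed to GetAttackTarget, which writes it to the blackboard's attack target key and stores it in the AttackTarget variable.
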(event EventBeginPlay
  (Class|AIController|UseBlackboard "/Game/assets/blueprints/AI/BB_Enemy.BB_Enemy")
  (AI|RunBehaviorTree "/Game/assets/blueprints/AI/BT_Enemy.BT_Enemy")
  (bind _asbp_player (Utilities|Casting|CastToBP_Player (Game|Player|GetPlayerPawn 0)))
  (CallFunction|GetAttackTarget _asbp_player))

(event EventTick
  (params (DeltaSeconds :type Float%20%28single-precision%29)))

(fn ConstructionScript)

(fn GetAttackTarget
  (params (AttackTarget :type BP%20Player%20Object%20Reference))
  (AI|Components|Blackboard|SetValueasObject (Variables|Default|GetBlackboard) (Variables|Default|GetAttack%20Target%20Key) AttackTarget)
  (Variables|Default|SetAttackTarget AttackTarget))